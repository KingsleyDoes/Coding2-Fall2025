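; Sewer dungeon door that swings open when the third-person character overlaps its box, optionally locked by a typed key.
; Unlocking requires a key and matching elemental type and spends one key; otherwise a temporary dialogue widget explains the refusal.
; A one-shot Timeline drives the yaw swing, registering the door in the game mode's save state.
; OpenThyself enters the same rotation-and-save step directly, without playing the Timeline.
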(event OnComponentBeginOverlap(Box)
  (params (OverlappedComponent :type Primitive%20Component%20Object%20Reference) (OtherActor :type Actor%20Object%20Reference) (OtherComp :type Primitive%20Component%20Object%20Reference) (OtherBodyIndex :type Integer) (bFromSweep :type Boolean) (SweepResult :type Hit%20Result%20Structure%20%28by%20ref%29))
  (bind _sm_door (Variables|Default|GetSM_Door))
  (bind _returnvalue (Transformation|GetWorldLocation _sm_door))
  (bind _asbp_third_person_character (Utilities|Casting|CastToBP_ThirdPersonCharacter OtherActor))
  (if (Variables|Default|GetLocked)
    (if (> (Variables|/Game/ThirdPerson/Blueprints/BP_ThirdPersonCharacter.BP_ThirdPersonCharacter_C|GetNumberOfKeys _asbp_third_person_character) 0)
      (if (Utilities|Enum|Equal(Enum) (Variables|/Game/ThirdPerson/Blueprints/BP_ThirdPersonCharacter.BP_ThirdPersonCharacter_C|GetElementalType _asbp_third_person_character) (Variables|Default|GetType))
        (Math|Integer|DecrementInt (Variables|/Game/ThirdPerson/Blueprints/BP_ThirdPersonCharacter.BP_ThirdPersonCharacter_C|GetNumberOfKeys _asbp_third_person_character)
          (:%20%20
            (Variables|Default|SetLocked false)))
        (else
          (Utilities|FlowControl|DoOnce false :!label _label
            (:Completed
              (bind _returnvalue_2 (UserInterface|CreateWidget "/Game/WidgetsUI/W_Dialogue.W_Dialogue_C" (Game|GetPlayerController 0)))
              (UserInterface|Viewport|AddtoViewport _returnvalue_2 0)
              (Variables|/Game/WidgetsUI/W_Dialogue.W_Dialogue_C|SetDialogue _returnvalue_2 "I Don't Have The Right Key For This Door.")
              (Utilities|FlowControl|Delay 5.0)
              (Widget|RemovefromParent _returnvalue_2)
              (goto _label Reset)))))
      (else
        (Utilities|FlowControl|DoOnce false :!label _label_2
          (:Completed
            (bind _returnvalue_3 (UserInterface|CreateWidget "/Game/WidgetsUI/W_Dialogue.W_Dialogue_C" (Game|GetPlayerController 0)))
            (UserInterface|Viewport|AddtoViewport _returnvalue_3 0)
            (Variables|/Game/WidgetsUI/W_Dialogue.W_Dialogue_C|SetDialogue _returnvalue_3 "It's Locked.")
            (Audio|PlaySoundatLocation "/Game/Audio/250041__underlineddesigns__gate-lock-slam.250041__underlineddesigns__gate-lock-slam" _returnvalue "0, 0, 0" 1.0 1.0 0.0 0 0 0 0)
            (Utilities|FlowControl|Delay 5.0)
            (Widget|RemovefromParent _returnvalue_3)
            (goto _label_2 Reset))))))
  (Utilities|FlowControl|DoOnce false
    (:Completed
      (Audio|PlaySoundatLocation "/Game/Audio/516009__wesleyextreme_gamer__gate-locked.516009__wesleyextreme_gamer__gate-locked" _returnvalue "0, 0, 0" 1.0 1.0 0.0 0 0 0 0)
      (bind _newtrack_0 (Timeline|Timeline PlayFromStart)
        (:Update
          (Transformation|SetRelativeRotation (Variables|Default|GetSM_Door) (Math|Rotator|MakeRotator 0.0 0.0 (Math|Float|Lerp 0.0 85.0 _newtrack_0)) false false)
          (CallFunction|AddtoSave))
        (:Finished)))))

(event Custom|OpenThyself
  (Transformation|SetRelativeRotation (Variables|Default|GetSM_Door) (Math|Rotator|MakeRotator 0.0 0.0 (Math|Float|Lerp 0.0 85.0 (stale OnComponentBeginOverlap(Box) _newtrack_0))) false false)
  (CallFunction|AddtoSave))

(event EventBeginPlay
  (|CallParentFunction) ; This node is disabled and will not be called.\nDrag off pins to build functionality.
)

(event Collision|EventActorBeginOverlap
  (params (OtherActor :type Actor%20Object%20Reference))
  (|CallParentFunction OtherActor) ; This node is disabled and will not be called.\nDrag off pins to build functionality.
)

(event EventTick
  (params (DeltaSeconds :type Float%20%28single-precision%29))
  (|CallParentFunction DeltaSeconds) ; This node is disabled and will not be called.\nDrag off pins to build functionality.
)

(event EventAddtoSave
  (bind _asgm_save_load (Utilities|Casting|CastToGM_SaveLoad (Game|GetGameMode)))
  (Utilities|Array|AddUnique (Variables|/Game/Blueprints/SaveAndLoad/SG_LevelState.SG_LevelState_C|GetInterfacedItems (Variables|/Game/Blueprints/SaveAndLoad/GM_SaveLoad.GM_SaveLoad_C|GetSG_LevelState _asgm_save_load)) self))

(fn ConstructionScript
  (|CallParentFunction))