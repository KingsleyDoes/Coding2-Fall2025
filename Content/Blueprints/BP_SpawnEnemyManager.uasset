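; BP_SpawnEnemyManager populates a level with randomized AI enemies when play begins.
; On BeginPlay it gathers every BP_EnemySpawnPoint, prints the count, and gives each a weighted, mostly favorable chance to spawn a BP_AiMoveTo at its transform, owned by that point.
; Each spawned enemy gets a random skeletal mesh, random materials on two slots, and a random name and color on its text render label.
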(event EventBeginPlay
  (bind _names (Variables|Default|GetNames))
  (bind _materials (Variables|Default|GetMaterials))
  (bind _outitem (Utilities|Array|Random _materials))
  (bind _outactors (Actor|GetAllActorsOfClass "/Game/Blueprints/BP_EnemySpawnPoint.BP_EnemySpawnPoint_C"))
  (Development|PrintText (Utilities|Text|FormatText "{points} spawn points in level" (Utilities|Array|Length _outactors)))
  (for _array_element _outactors
    (if (Math|Random|RandomBoolwithWeight 0.75)
      (bind _returnvalue (Game|SpawnActorfromClass "/Game/AI_Blueprints/BP_AiMoveTo.BP_AiMoveTo_C" (Transformation|GetActorTransform _array_element) "Undefined" "MultiplyWithRoot" _array_element 0))
      (Utilities|Array|Shuffle _names)
      (Rendering|Components|TextRender|SetText (Variables|/Game/AI_Blueprints/BP_AiMoveTo.BP_AiMoveTo_C|Gettextrender%20Name _returnvalue) (.OutItem (Utilities|Array|Random _names)))
      (Components|SkeletalMesh|SetSkeletalMeshAsset (Variables|/Script/Engine.Character|GetMesh _returnvalue) (.OutItem (Utilities|Array|Random (Variables|Default|GetSkeletal%20Mesh%20Assets))))
      (Rendering|Material|SetMaterial (Variables|/Script/Engine.Character|GetMesh _returnvalue) 0 _outitem)
      (Rendering|Material|SetMaterial (Variables|/Script/Engine.Character|GetMesh _returnvalue) 1 _outitem) ; add an array of materials
      (Rendering|Components|TextRender|SetTextRenderColor (Variables|/Game/AI_Blueprints/BP_AiMoveTo.BP_AiMoveTo_C|Gettextrender%20Name _returnvalue) (.OutItem (Utilities|Array|Random (Variables|Default|GetTextcolor)))))))

(fn ConstructionScript)