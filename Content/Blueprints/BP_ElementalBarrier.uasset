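; Elemental barrier actor that only lets the third-person character through when its elemental type matches the barrier's.
; On begin play, a text render labels it with its type name.
; When the character overlaps the collision component, a type match turns off the barrier's collision, while a mismatch restores blocking collision and prints a refusal message.
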(event OnComponentBeginOverlap(Collision)
  (params (OverlappedComponent :type Primitive%20Component%20Object%20Reference) (OtherActor :type Actor%20Object%20Reference) (OtherComp :type Primitive%20Component%20Object%20Reference) (OtherBodyIndex :type Integer) (bFromSweep :type Boolean) (SweepResult :type Hit%20Result%20Structure%20%28by%20ref%29))
  (bind _barrier (Variables|Default|GetBarrier))
  (bind _asbp_third_person_character (Utilities|Casting|CastToBP_ThirdPersonCharacter OtherActor))
  (if (Utilities|Enum|Equal(Enum) (Variables|/Game/ThirdPerson/Blueprints/BP_ThirdPersonCharacter.BP_ThirdPersonCharacter_C|GetElementalType _asbp_third_person_character) (Variables|Default|GetElementalType))
    (Collision|SetCollisionEnabled _barrier "NoCollision")
    (else
      (Development|PrintText (Utilities|Text|FormatText "You can't get in here while you still have the wrong type."))
      (Collision|SetCollisionEnabled _barrier "QueryAndPhysics"))))

(event EventBeginPlay
  (Rendering|Components|TextRender|SetText (Variables|Default|GetTextRender) (Utilities|Text|FormatText "{type} Barrier" (|GenerictoText (Variables|Default|GetElementalType)))))

(event Collision|EventActorBeginOverlap
  (params (OtherActor :type Actor%20Object%20Reference)))

(event EventTick
  (params (DeltaSeconds :type Float%20%28single-precision%29)))

(fn ConstructionScript)