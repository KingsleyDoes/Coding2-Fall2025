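; Character weapon pickup, an axe, that equips onto the player and enables attacking.
; Pickup sets the character's weapon flags, snaps the axe to a hand socket, disables box collision and records the item and unlock in GM_SaveLoad.
; In Final-Lvl2 it also plays a pickup sound and timed dialogue with a swing hint.
; The primary and secondary use events are effectively empty stubs.
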(event EventPickup
  (params (Skeletal%20Mesh :type Skeletal%20Mesh%20Component%20Object%20Reference))
  (bind _returnvalue (Game|GetCurrentLevelName true))
  (if (Utilities|Enum|Equal(Enum) _returnvalue "Final-Lvl2")
    (Utilities|FlowControl|Sequence
      (:then_0
        (bind _asbp_third_person_character (Utilities|Casting|CastToBP_ThirdPersonCharacter (Game|GetPlayerCharacter 0) :!label _label))
        (Variables|/Game/ThirdPerson/Blueprints/BP_ThirdPersonCharacter.BP_ThirdPersonCharacter_C|SetWeaponEquipped _asbp_third_person_character true)
        (bind _returnvalue_2 (Actor|GetActorOfClass "/Game/ThirdPerson/Blueprints/BP_ThirdPersonCharacter.BP_ThirdPersonCharacter_C"))
        (Variables|/Game/ThirdPerson/Blueprints/BP_ThirdPersonCharacter.BP_ThirdPersonCharacter_C|SetCanAttack _returnvalue_2 true)
        (Transformation|AttachComponentToComponent Skeletal%20Mesh "index_03_rSocket" "SnapToTarget" "SnapToTarget" "SnapToTarget" true)
        (Collision|SetCollisionEnabled (Variables|Default|GetBox) "NoCollision")
        (CallFunction|AddtoSave)
        (CallFunction|AddtoSave))
      (:then_1
        (Audio|PlaySound2D "/Game/WidgetsUI/Sound/C_AxePickup.C_AxePickup" 1.0 1.0 0.0 0 0)
        (Utilities|FlowControl|Delay 2.0)
        (bind _returnvalue_3 (UserInterface|CreateWidget "/Game/WidgetsUI/W_Dialogue.W_Dialogue_C" (Game|GetPlayerController 0)))
        (UserInterface|Viewport|AddtoViewport _returnvalue_3 0)
        (Variables|/Game/WidgetsUI/W_Dialogue.W_Dialogue_C|SetDialogue _returnvalue_3 "My Axe! What's It Doing Down Here?")
        (Utilities|FlowControl|Delay 3.0)
        (Widget|RemovefromParent _returnvalue_3))
      (:then_2
        (Utilities|FlowControl|Delay 6.0)
        (bind _returnvalue_4 (UserInterface|CreateWidget "/Game/WidgetsUI/W_Dialogue.W_Dialogue_C" (Game|GetPlayerController 0)))
        (UserInterface|Viewport|AddtoViewport _returnvalue_4 0)
        (Variables|/Game/WidgetsUI/W_Dialogue.W_Dialogue_C|SetDialogue _returnvalue_4 "Press Middle Mouse Button To Swing.")
        (Utilities|FlowControl|Delay 5.0)
        (Widget|RemovefromParent _returnvalue_4)))
    (else
      (goto _label))))

(event EventUsePrimary)

(event EventUseSecondary
  (Utilities|FlowControl|FlipFlop))

(event EventAddtoSave
  (bind _asgm_save_load (Utilities|Casting|CastToGM_SaveLoad (Game|GetGameMode)))
  (Utilities|Array|AddUnique (Variables|/Game/Blueprints/SaveAndLoad/SG_LevelState.SG_LevelState_C|GetInterfacedItems (Variables|/Game/Blueprints/SaveAndLoad/GM_SaveLoad.GM_SaveLoad_C|GetSG_LevelState _asgm_save_load)) self)
  (Variables|/Game/Blueprints/SaveAndLoad/GM_SaveLoad.GM_SaveLoad_C|SetWeapon%20Unlocked _asgm_save_load true))

(fn ConstructionScript)