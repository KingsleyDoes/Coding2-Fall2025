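; BP_Ward is a held pickup whose primary use plays a sound and switches every enemy's AI controller to the first state of its enum with a zeroed point of interest.
; Pickup snaps it to a left-hand finger socket on the given skeletal mesh and disables collision on its box and cylinder.
; Drop detaches it and restores collision, simulating physics for a short delay before freezing it again.
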(event EventBeginPlay)

(event Collision|EventActorBeginOverlap
  (params (OtherActor :type Actor%20Object%20Reference)))

(event EventTick
  (params (DeltaSeconds :type Float%20%28single-precision%29)))

(event EventPickup
  (params (Skeletal%20Mesh :type Skeletal%20Mesh%20Component%20Object%20Reference))
  (Development|PrintText "This item got picked up")
  (Transformation|AttachComponentToComponent Skeletal%20Mesh "ring_02_l" "SnapToTarget" "SnapToTarget" "KeepRelative" true)
  (Collision|SetCollisionEnabled (Variables|Default|GetBox) "NoCollision"))

(event EventUsePrimary
  (Audio|PlaySound2D "/Game/Audio/409259__wertstahl__003.409259__wertstahl__003" 1.0 1.0 0.0 0 0)
  (bind _outactors (Actor|GetAllActorsOfClass "/Game/AI_Blueprints/BP_EnemyBase.BP_EnemyBase_C"))
  (for _array_element _outactors
    (Utilities|IsValid _array_element
      (:Is%20Valid
        (bind _asaic_enemy_base (Utilities|Casting|CastToAIC_EnemyBase (AI|GetAIController _array_element)))
        (Default|SetState _asaic_enemy_base "NewEnumerator0" 0 "0, 0, 0")))))

(event EventUseSecondary)

(event EventDrop
  (Transformation|DetachFromActor "KeepWorld" "KeepWorld" "KeepRelative")
  (Physics|SetSimulatePhysics (Variables|Default|GetCylinder) true)
  (Collision|SetCollisionEnabled (Variables|Default|GetBox) "QueryAndPhysics")
  (Utilities|FlowControl|Delay 2.0)
  (Physics|SetSimulatePhysics (Variables|Default|GetCylinder) false))

(fn ConstructionScript)