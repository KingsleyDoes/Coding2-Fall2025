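; Ankle monitor pickup that, on Pickup, snaps to the left foot IK socket of the given skeletal mesh and disables its box collision.
; Primary and secondary use each drive a FlipFlop on player 0's character movement, toggling doubled walk speed and doubled gravity respectively.
; Drop destroys the actor without restoring either movement value, and each action prints a message.
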(event EventBeginPlay)

(event Collision|EventActorBeginOverlap
  (params (OtherActor :type Actor%20Object%20Reference)))

(event EventTick
  (params (DeltaSeconds :type Float%20%28single-precision%29)))

(event EventPickup
  (params (Skeletal%20Mesh :type Skeletal%20Mesh%20Component%20Object%20Reference))
  (Development|PrintText "This ankle monitor got picked up")
  (Transformation|AttachComponentToComponent Skeletal%20Mesh "ik_foot_l" "SnapToTarget" "SnapToTarget" "SnapToTarget" true)
  (Collision|SetCollisionEnabled (Variables|Default|GetBox) "NoCollision"))

(event EventUsePrimary
  (bind _returnvalue (Game|GetPlayerCharacter 0))
  (bind _charactermovement (Variables|/Script/Engine.Character|GetCharacterMovement _returnvalue))
  (Development|PrintText "Toggled speed boost")
  (Utilities|FlowControl|FlipFlop
    (:A
      (Variables|/Script/Engine.CharacterMovementComponent|SetMaxWalkSpeed _charactermovement 1.2e+03))
    (:B
      (Variables|/Script/Engine.CharacterMovementComponent|SetMaxWalkSpeed _charactermovement 6e+02))))

(event EventUseSecondary
  (bind _returnvalue (Game|GetPlayerCharacter 0))
  (bind _charactermovement (Variables|/Script/Engine.Character|GetCharacterMovement _returnvalue))
  (Development|PrintText "Toggled ankle weight")
  (Utilities|FlowControl|FlipFlop
    (:A
      (Variables|/Script/Engine.CharacterMovementComponent|SetGravityScale _charactermovement 2.0))
    (:B
      (Variables|/Script/Engine.CharacterMovementComponent|SetGravityScale _charactermovement 1.0))))

(event EventDrop
  (Development|PrintString "You dropped the ankle monitor")
  (Actor|DestroyActor))

(fn ConstructionScript)