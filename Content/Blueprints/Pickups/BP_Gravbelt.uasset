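; BP_Gravbelt is a gravity belt pickup that snaps to the spine_02 socket of the supplied skeletal mesh and disables its box collision when picked up.
; Primary and secondary use each drive a FlipFlop on player 0's CharacterMovement, toggling a higher jump velocity and a low-gravity slowfall.
; Drop destroys the actor without restoring either movement value, and each action prints a message.
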(event EventBeginPlay)

(event Collision|EventActorBeginOverlap
  (params (OtherActor :type Actor%20Object%20Reference)))

(event EventTick
  (params (DeltaSeconds :type Float%20%28single-precision%29)))

(event EventPickup
  (params (Skeletal%20Mesh :type Skeletal%20Mesh%20Component%20Object%20Reference))
  (Development|PrintText "This belt got picked up")
  (Transformation|AttachComponentToComponent Skeletal%20Mesh "spine_02" "SnapToTarget" "SnapToTarget" "SnapToTarget" true)
  (Collision|SetCollisionEnabled (Variables|Default|GetBox) "NoCollision"))

(event EventUsePrimary
  (bind _returnvalue (Game|GetPlayerCharacter 0))
  (bind _charactermovement (Variables|/Script/Engine.Character|GetCharacterMovement _returnvalue))
  (Development|PrintText "Toggled jump height")
  (Utilities|FlowControl|FlipFlop
    (:A
      (Variables|/Script/Engine.CharacterMovementComponent|SetJumpZVelocity _charactermovement 1e+03))
    (:B
      (Variables|/Script/Engine.CharacterMovementComponent|SetJumpZVelocity _charactermovement 5e+02))))

(event EventUseSecondary
  (bind _returnvalue (Game|GetPlayerCharacter 0))
  (bind _charactermovement (Variables|/Script/Engine.Character|GetCharacterMovement _returnvalue))
  (Development|PrintText "Toggled slowfall")
  (Utilities|FlowControl|FlipFlop
    (:A
      (Variables|/Script/Engine.CharacterMovementComponent|SetGravityScale _charactermovement 0.25))
    (:B
      (Variables|/Script/Engine.CharacterMovementComponent|SetGravityScale _charactermovement 1.0))))

(event EventDrop
  (Development|PrintString "You dropped the gravbelt")
  (Actor|DestroyActor))

(fn ConstructionScript)