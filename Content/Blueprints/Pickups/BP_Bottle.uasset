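; BP_Bottle is a throwable pickup that shows a tutorial widget when the player overlaps it and attaches to a hand socket when picked up.
; Primary use plays a hook montage, then traces along the camera's forward vector from the character, and a timeline lerps the mesh to the impact point.
; The throw ends in glass sound, Niagara shards and destruction.
; Throwing and dropping both report noise events, and dropping breaks it in place.
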(event OnComponentBeginOverlap(Box)
  (params (OverlappedComponent :type Primitive%20Component%20Object%20Reference) (OtherActor :type Actor%20Object%20Reference) (OtherComp :type Primitive%20Component%20Object%20Reference) (OtherBodyIndex :type Integer) (bFromSweep :type Boolean) (SweepResult :type Hit%20Result%20Structure%20%28by%20ref%29))
  (Utilities|Casting|CastToBP_ThirdPersonCharacter OtherActor)
  (bind _returnvalue (UserInterface|CreateWidget "/Game/WidgetsUI/W_Tut.W_Tut_C" (Game|GetPlayerController 0)))
  (bind _output_get (Variables|Default|SetWidget _returnvalue))
  (UserInterface|Viewport|AddtoPlayerScreen _output_get))

(event OnComponentEndOverlap(Box)
  (params (OverlappedComponent :type Primitive%20Component%20Object%20Reference) (OtherActor :type Actor%20Object%20Reference) (OtherComp :type Primitive%20Component%20Object%20Reference) (OtherBodyIndex :type Integer))
  (Utilities|Casting|CastToBP_ThirdPersonCharacter OtherActor)
  (Widget|RemovefromParent (Variables|Default|GetWidget)))

(event EventBeginPlay)

(event Collision|EventActorBeginOverlap
  (params (OtherActor :type Actor%20Object%20Reference)))

(event EventTick
  (params (DeltaSeconds :type Float%20%28single-precision%29)))

(event EventPickup
  (params (Skeletal%20Mesh :type Skeletal%20Mesh%20Component%20Object%20Reference))
  (Development|PrintText "This bottle got picked up")
  (Transformation|AttachComponentToComponent Skeletal%20Mesh "ring_02_l" "SnapToTarget" "SnapToTarget" "KeepWorld" true)
  (Collision|SetCollisionEnabled (Variables|Default|GetBox) "NoCollision"))

(event EventUsePrimary
  (bind _asbp_third_person_character (Utilities|Casting|CastToBP_ThirdPersonCharacter (Game|GetPlayerCharacter 0)))
  (Animation|PlayAnimMontage _asbp_third_person_character "/Game/CloseCombatAnimSet/Animations/InPlace/Attacks/AM_LeftHook.AM_LeftHook" 1.0 "None")
  (Utilities|FlowControl|Delay 0.7)
  (bind _outhit (Collision|LineTraceByChannel (Transformation|GetActorLocation _asbp_third_person_character) (+ (* (Math|Vector|GetForwardVector (Variables|/Game/ThirdPerson/Blueprints/BP_ThirdPersonCharacter.BP_ThirdPersonCharacter_C|GetFollowCamera _asbp_third_person_character)) 1e+04) (Transformation|GetActorLocation _asbp_third_person_character)) "TraceTypeQuery2" false (Utilities|Array|MakeArray _asbp_third_person_character) "Persistent"))
  (bind _newtrack_0 (Timeline|Throw Play)
    (:Update
      (Transformation|SetWorldLocation (Variables|Default|GetCylinder) (Math|Vector|Lerp(Vector) (Transformation|GetWorldLocation (Variables|Default|GetCylinder)) (.ImpactPoint (Collision|BreakHitResult _outhit)) _newtrack_0) false false))
    (:Finished
      (Audio|PlaySoundatLocation "/Game/WidgetsUI/Sound/C_Glass.C_Glass" (.ImpactPoint (Collision|BreakHitResult _outhit)) "0, 0, 0" 1.0 1.0 0.0 0 0 0 0)
      (Niagara|SpawnSystematLocation "/Game/VFX/NS_BottleShards.NS_BottleShards" (.ImpactPoint (Collision|BreakHitResult _outhit)))
      (Actor|DestroyActor))
    (:NewTrack_1
      (Class|AISenseHearing|ReportNoiseEvent (.ImpactPoint (Collision|BreakHitResult _outhit)) 1e+01 0 0.0 "Noise"))))

(event EventDrop
  (bind _returnvalue (Transformation|GetActorLocation))
  (Audio|PlaySoundatLocation "/Game/WidgetsUI/Sound/C_Glass.C_Glass" _returnvalue "0, 0, 0" 1.0 1.0 0.0 0 0 0 0)
  (Class|AISenseHearing|ReportNoiseEvent _returnvalue 1e+01 0 0.0 "Noise")
  (Actor|DestroyActor))

(fn ConstructionScript)