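; Game mode that saves and restores per-level state and player stats through SaveGame objects.
; On BeginPlay it loads or creates SG_LevelState in a slot named after the level, replaying saved coins, doors and interfaced items; the weapon branch only casts.
; It also loads or creates SG_PlayerStats in "PlayerSave", restoring Health but setting Mana from the held item.
; Separate events write both saves and print results; stamina restoration is disconnected.
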(event Custom|SaveLevelStateToFile
  (bind _returnvalue (Game|GetCurrentLevelName true))
  (bind _returnvalue_2 (SaveGame|SaveGametoSlot (Variables|Default|GetSG_LevelState) _returnvalue))
  (if _returnvalue_2
    (Development|PrintText "Level state saved" true true "(R=0.261434,G=0.594792,B=0.067534,A=1.000000)" 5.0)
    (else
      (Development|PrintText "Level state save error" true true "(R=0.753125,G=0.000000,B=0.018387,A=1.000000)" 15.0))))

(event Custom|Load%20Level%20State%20From%20File
  (bind _returnvalue (Game|GetCurrentLevelName true))
  (bind _returnvalue_2 (SaveGame|DoesSaveGameExist _returnvalue))
  (if _returnvalue_2
    (bind _returnvalue_3 (SaveGame|LoadGamefromSlot _returnvalue))
    (bind _assg_level_state (Utilities|Casting|CastToSG_LevelState _returnvalue_3))
    (Variables|Default|SetSG_LevelState _assg_level_state)
    (Utilities|FlowControl|Sequence
      (:then_0
        ;[0.15 0.15 0.15 0.5] load collected coins
        (for _array_element (Variables|/Game/Blueprints/SaveAndLoad/SG_LevelState.SG_LevelState_C|GetCollectedCoins (Variables|Default|GetSG_LevelState))
          (Utilities|IsValid _array_element
            (:Is%20Valid
              (Default|CollectThyself _array_element)))))
      (:then_1
        ;[0.15 0.15 0.15 0.5] load opened doors
        (for _array_element_2 (Variables|/Game/Blueprints/SaveAndLoad/SG_LevelState.SG_LevelState_C|GetOpenedDoors (Variables|Default|GetSG_LevelState))
          (Utilities|IsValid _array_element_2
            (:Is%20Valid
              (Default|QuietOpen _array_element_2)))))
      (:then_2
        ;[0.15 0.15 0.15 0.5] Interfaced Items
        (for _array_element_3 (Variables|/Game/Blueprints/SaveAndLoad/SG_LevelState.SG_LevelState_C|GetInterfacedItems (Variables|Default|GetSG_LevelState))
          (Utilities|FlowControl|Sequence
            (:then_0
              (if (== _array_element_3 "/Game/Blueprints/BP_Key.BP_Key")
                (bind _asbp_key (Utilities|Casting|CastToBP_Key _array_element_3))
                (Default|PickupThyself _asbp_key)))
            (:then_1
              (if (== _array_element_3 "/Game/Medieval_Sewer_Dungeon/Blueprints/Props/BP_Door.BP_Door")
                (bind _asbp_door (Utilities|Casting|CastToBP_Door _array_element_3))
                (Default|OpenThyself _asbp_door)))
            (:then_2
              (if (== _array_element_3 "/Game/Blueprints/Pickups/BP_CharacterWeapon.BP_CharacterWeapon")
                (Utilities|Casting|CastToBP_CharacterWeapon _array_element_3)))))))
    (else
      (bind _returnvalue_4 (SaveGame|CreateSaveGameObject "/Game/Blueprints/SaveAndLoad/SG_LevelState.SG_LevelState_C"))
      (Variables|Default|SetSG_LevelState _returnvalue_4))))

(event Custom|LoadPlayerStats
  (bind _returnvalue (SaveGame|DoesSaveGameExist "PlayerSave"))
  (if _returnvalue
    (bind _returnvalue_2 (SaveGame|LoadGamefromSlot "PlayerSave"))
    (bind _assg_player_stats (Utilities|Casting|CastToSG_PlayerStats _returnvalue_2))
    (Variables|Default|SetSG_PlayerStats _assg_player_stats)
    (bind _asbp_third_person_character (Utilities|Casting|CastToBP_ThirdPersonCharacter (Game|GetPlayerCharacter 0)))
    (Utilities|FlowControl|Sequence
      (:then_0
        (Variables|/Game/ThirdPerson/Blueprints/BP_ThirdPersonCharacter.BP_ThirdPersonCharacter_C|SetHealth _asbp_third_person_character (Variables|/Game/Blueprints/SaveAndLoad/SG_PlayerStats.SG_PlayerStats_C|GetHealth (Variables|Default|GetSG_PlayerStats))))
      (:then_1
        (if (== (Variables|/Game/ThirdPerson/Blueprints/BP_ThirdPersonCharacter.BP_ThirdPersonCharacter_C|GetHeldItem _asbp_third_person_character) "/Game/Blueprints/Pickups/BP_CharacterWeapon.BP_CharacterWeapon")
          (Variables|/Game/ThirdPerson/Blueprints/BP_ThirdPersonCharacter.BP_ThirdPersonCharacter_C|SetMana _asbp_third_person_character 1.0)
          (else
            (Variables|/Game/ThirdPerson/Blueprints/BP_ThirdPersonCharacter.BP_ThirdPersonCharacter_C|SetMana _asbp_third_person_character 0.0)))))
    (else
      (bind _returnvalue_3 (SaveGame|CreateSaveGameObject "/Game/Blueprints/SaveAndLoad/SG_PlayerStats.SG_PlayerStats_C"))
      (bind _output_get (Variables|Default|SetSG_PlayerStats _returnvalue_3))
      (SaveGame|SaveGametoSlot _output_get "PlayerSave"))))

(event Custom|SavePlayerStats
  (bind _returnvalue (SaveGame|DoesSaveGameExist "PlayerSave"))
  (if _returnvalue
    (bind _returnvalue_2 (SaveGame|SaveGametoSlot (Variables|Default|GetSG_PlayerStats) "PlayerSave"))
    (if _returnvalue_2
      (Development|PrintText "Stats successfully written to file" true true "(R=1.000000,G=0.206482,B=0.000000,A=1.000000)")
      (else
        (Development|PrintText "Failure to write stats to file" true true "(R=0.430490,G=0.000000,B=1.000000,A=1.000000)" 5.0)))
    (else
      (Development|PrintText "No save game found"))))

(event EventBeginPlay
  (CallFunction|LoadLevelStatefromFile)
  (CallFunction|LoadPlayerStats))

(fn ConstructionScript)