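; BP_SwordCheck is a trigger box that hands the character weapon to the player on overlap.
; When a BP_ThirdPersonCharacter enters the box, it finds a BP_CharacterWeapon in the level with GetActorOfClass and calls Pickup with the character's mesh.
; An unconnected branch holds save-based equip logic that checks WeaponEquipped and GM_SaveLoad's InterfacedItems, plus debug prints; it never runs.
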(event OnComponentBeginOverlap(Box)
  (params (OverlappedComponent :type Primitive%20Component%20Object%20Reference) (OtherActor :type Actor%20Object%20Reference) (OtherComp :type Primitive%20Component%20Object%20Reference) (OtherBodyIndex :type Integer) (bFromSweep :type Boolean) (SweepResult :type Hit%20Result%20Structure%20%28by%20ref%29))
  (bind _asbp_third_person_character (Utilities|Casting|CastToBP_ThirdPersonCharacter OtherActor))
  (bind _returnvalue (Actor|GetActorOfClass "/Game/Blueprints/Pickups/BP_CharacterWeapon.BP_CharacterWeapon_C"))
  (Default|Pickup _returnvalue (Variables|/Script/Engine.Character|GetMesh _asbp_third_person_character)))

(fn ConstructionScript)