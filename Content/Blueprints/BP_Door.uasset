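; A door that slides down when the third-person character enters its trigger sphere, using up one of the character's keys if locked.
; The Drop timeline lerps the door's height, with a delayed reverse triggered from its update to raise it again.
; DoOnce gates block retriggering until the timeline finishes and throttle the on-screen locked message shown to players without keys.
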(event OnComponentBeginOverlap(Sphere)
  (params (OverlappedComponent :type Primitive%20Component%20Object%20Reference) (OtherActor :type Actor%20Object%20Reference) (OtherComp :type Primitive%20Component%20Object%20Reference) (OtherBodyIndex :type Integer) (bFromSweep :type Boolean) (SweepResult :type Hit%20Result%20Structure%20%28by%20ref%29))
  (bind _asbp_third_person_character (Utilities|Casting|CastToBP_ThirdPersonCharacter OtherActor))
  (if (Variables|Default|GetLocked)
    (if (> (Variables|/Game/ThirdPerson/Blueprints/BP_ThirdPersonCharacter.BP_ThirdPersonCharacter_C|GetNumberOfKeys _asbp_third_person_character) 0)
      (Math|Integer|DecrementInt (Variables|/Game/ThirdPerson/Blueprints/BP_ThirdPersonCharacter.BP_ThirdPersonCharacter_C|GetNumberOfKeys _asbp_third_person_character)
        (:%20%20
          (Development|PrintString "This door is now unlocked" true true "(R=1.000000,G=0.284375,B=0.499461,A=1.000000)")
          (Variables|Default|SetLocked false)))
      (else
        (Utilities|FlowControl|DoOnce false :!label _label
          (:Completed
            (Development|PrintString "Looks like it's locked" true true "(R=1.000000,G=0.284375,B=0.499461,A=1.000000)")
            (Utilities|FlowControl|Delay 5.0)
            (goto _label Reset))))))
  (Utilities|FlowControl|DoOnce false :!label _label_2
    (:Completed
      (bind _newtrack_0 (Timeline|Drop PlayFromStart)
        (:Update
          (Transformation|SetRelativeLocation (Variables|Default|Getdoor) (Math|Vector|MakeVector 0.0 0.0 (Math|Float|Lerp 2.5e+02 -2.4e+02 _newtrack_0)) false false)
          (Utilities|FlowControl|Delay 5.0)
          (Timeline|Drop ReverseFromEnd))
        (:Finished
          (goto _label_2 Reset))))))

(event EventBeginPlay)

(event Collision|EventActorBeginOverlap
  (params (OtherActor :type Actor%20Object%20Reference)))

(event EventTick
  (params (DeltaSeconds :type Float%20%28single-precision%29)))

(fn ConstructionScript)