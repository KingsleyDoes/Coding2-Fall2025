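; Demo Blueprint of loop constructs and arrays, printing iteration counts as plain and colored on-screen text.
; DelayLoop re-calls itself through a one-second Delay and a DoN cap, running the indexed-color ForLoop on each pass.
; Separate events show a counter-driven WhileLoop that resets afterwards and a ForEach over a color array.
; BeginPlay is empty and the chains calling DelayLoop, WhileLoop and ForEach from outside are disconnected, so nothing starts.
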(event Custom|DelayLoop
  (Development|PrintString (Utilities|String|Append "This string has run " (Utilities|String|ToString(Integer) (stale _counter)) " times."))
  (Development|PrintText (Utilities|Text|FormatText "This text has run {count} times." (stale _counter)) true true "(R=1.000000,G=0.660000,B=1.000000,A=1.000000)") ; Does the same thing as the print string + append, just with a different layout.
  (Utilities|FlowControl|Delay 1.0)
  (bind _counter (Utilities|FlowControl|DoN 20)
    (:Exit
      (CallFunction|StartforLoop)
      (CallFunction|DelayLoop))))

(event Custom|StartForLoop
  (bind _array (Utilities|Array|MakeArray "(R=1.000000,G=0.000000,B=0.669804,A=1.000000)" "(R=1.000000,G=0.549212,B=0.000000,A=1.000000)" "(R=1.000000,G=0.206482,B=0.000000,A=1.000000)" "(R=1.000000,G=0.000000,B=0.108982,A=1.000000)" "(R=0.430491,G=0.000000,B=1.000000,A=1.000000)" "(R=0.000000,G=0.233146,B=1.000000,A=1.000000)"))
  (for _index (range 0 (- (Utilities|Array|Length _array) 1) 2)
    (Development|PrintText (Utilities|Text|FormatText "For Loop has run {index} times" _index) true true (Utilities|Array|Get(acopy) _array _index))))

(event Custom|StartWhileLoop
  (while (> (Variables|Default|GetWhileLoopCounter) 0)
    (Development|PrintText (Utilities|Text|FormatText "There are {uses} more uses in this loop." (Variables|Default|GetWhileLoopCounter)) true true "(R=0.433680,G=1.000000,B=0.224121,A=1.000000)")
    (Math|Integer|DecrementInt (Variables|Default|GetWhileLoopCounter)))
  (Variables|Default|SetWhileLoopCounter 10))

(event Custom|StartForEachLoop
  (for (_array_element _array_index) (Utilities|Array|MakeArray "(R=1.000000,G=0.000000,B=0.669804,A=1.000000)" "(R=1.000000,G=0.549212,B=0.000000,A=1.000000)" "(R=1.000000,G=0.206482,B=0.000000,A=1.000000)" "(R=1.000000,G=0.000000,B=0.108982,A=1.000000)")
    (Development|PrintText (Utilities|Text|FormatText "For Each Loop has run {index} times." _array_index) true true _array_element)))

(event EventBeginPlay)

(fn ConstructionScript)