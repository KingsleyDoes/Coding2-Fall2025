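; Key pickup that raises BP_ThirdPersonCharacter's key count on sphere overlap and changes its elemental type.
; Pickup plays sound, reports noise, records itself in GM_SaveLoad and shows random dialogue for five seconds before applying the element and self-destructing.
; It also issues AIMoveTo on every enemy, targeting the enemy itself, and sets AI state on failure.
; PickupThyself destroys it directly; the egg's bob and spin timelines are unconnected.
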(event OnComponentBeginOverlap(Sphere)
  (params (OverlappedComponent :type Primitive%20Component%20Object%20Reference) (OtherActor :type Actor%20Object%20Reference) (OtherComp :type Primitive%20Component%20Object%20Reference) (OtherBodyIndex :type Integer) (bFromSweep :type Boolean) (SweepResult :type Hit%20Result%20Structure%20%28by%20ref%29))
  (bind _defaultsceneroot (Variables|Default|GetDefaultSceneRoot))
  (bind _returnvalue (Transformation|GetWorldLocation _defaultsceneroot))
  (bind _asbp_third_person_character (Utilities|Casting|CastToBP_ThirdPersonCharacter OtherActor))
  (Utilities|FlowControl|Sequence
    (:then_0
      (Math|Integer|IncrementInt (Variables|/Game/ThirdPerson/Blueprints/BP_ThirdPersonCharacter.BP_ThirdPersonCharacter_C|GetNumberOfKeys _asbp_third_person_character)
        (:%20%20
          (Audio|PlaySoundatLocation "/Game/WidgetsUI/Sound/C_KeyPickup.C_KeyPickup" _returnvalue "0, 0, 0" 1.0 1.0 0.0 0 0 0 0)
          (Class|AISenseHearing|ReportNoiseEvent _returnvalue 1.0 0 0.0 "None")
          (bind _returnvalue_2 (UserInterface|CreateWidget "/Game/WidgetsUI/W_Dialogue.W_Dialogue_C" (Game|GetPlayerController 0)))
          (UserInterface|Viewport|AddtoViewport _returnvalue_2 0)
          (Variables|/Game/WidgetsUI/W_Dialogue.W_Dialogue_C|SetDialogue _returnvalue_2 (.OutItem (Utilities|Array|Random (Variables|Default|GetDialogueOptions))))
          (CallFunction|AddtoSave)
          (CallFunction|AddtoSave)
          (Rendering|ToggleVisibility (Variables|Default|Getegg) false)
          (Utilities|FlowControl|Delay 5.0)
          (Widget|RemovefromParent _returnvalue_2)
          (if (Utilities|Enum|Equal(Enum) (Variables|/Game/ThirdPerson/Blueprints/BP_ThirdPersonCharacter.BP_ThirdPersonCharacter_C|GetElementalType _asbp_third_person_character) "NewEnumerator2")
            (Variables|/Game/ThirdPerson/Blueprints/BP_ThirdPersonCharacter.BP_ThirdPersonCharacter_C|SetElementalType _asbp_third_person_character "NewEnumerator4")
            (else
              (Variables|/Game/ThirdPerson/Blueprints/BP_ThirdPersonCharacter.BP_ThirdPersonCharacter_C|SetElementalType _asbp_third_person_character (Variables|Default|Gettype))))
          (Actor|DestroyActor))))
    (:then_1
      (bind _outactors (Actor|GetAllActorsOfClass "/Game/AI_Blueprints/BP_EnemyBase.BP_EnemyBase_C"))
      (for _array_element _outactors
        (bind _asaic_enemy_base (Utilities|Casting|CastToAIC_EnemyBase (Pawn|GetController _array_element)))
        (AI|AIMoveTo _asaic_enemy_base _returnvalue _array_element -1.0 "Default" "Default" true true
          (:OnRequestFailed
            (Default|SetState _asaic_enemy_base "NewEnumerator1" (Game|GetPlayerCharacter 0) "0, 0, 0")))))))

(event Custom|BobAndSpin)

(event Custom|PickupThyself
  (Actor|DestroyActor))

(event Collision|EventActorBeginOverlap
  (params (OtherActor :type Actor%20Object%20Reference)))

(event EventTick
  (params (DeltaSeconds :type Float%20%28single-precision%29)))

(event EventAddtoSave
  (bind _asgm_save_load (Utilities|Casting|CastToGM_SaveLoad (Game|GetGameMode)))
  (Utilities|Array|AddUnique (Variables|/Game/Blueprints/SaveAndLoad/SG_LevelState.SG_LevelState_C|GetInterfacedItems (Variables|/Game/Blueprints/SaveAndLoad/GM_SaveLoad.GM_SaveLoad_C|GetSG_LevelState _asgm_save_load)) self))

(fn ConstructionScript)