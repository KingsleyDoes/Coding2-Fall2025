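; Base enemy character for AI, providing aggro, attack, patrol, walk speed and range functions.
; Aggro toggles a flag and red body material, while attacks play a montage and signal completion even when interrupted.
; Patrol queries step along a spline route's points, reversing direction at the ends.
; Point damage reduces health, and at zero physics simulation, a radial impulse derived from shot direction and disabled movement create a ragdoll death.
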(event Custom|Attack
  ;[0.15 0.15 0.15 0.5] Attack player
  (Development|PrintText "AAAAAGH")
  (Animation|Montage|PlayMontage (Variables|Character|GetMesh) (Variables|Default|GetAttackMontage)
    (:OnCompleted
      _)
    (:OnInterrupted
      _))
  (Default|CallAttackFInished))

(event Custom|GetAg
  ;[0.15 0.15 0.15 0.5] We got beef
  (Rendering|Material|SetMaterial (Variables|Character|GetMesh) 0 "/AnimationSharing/AnimSharingRed.AnimSharingRed")
  (Variables|Default|SetAg true))

(event Custom|LoseAg
  ;[0.15 0.15 0.15 0.5] Beef squashed
  (Rendering|Material|SetMaterial (Variables|Character|GetMesh) 0 (Variables|Default|GetOriginalMat))
  (Variables|Default|SetAg false))

(event Custom|SetWalkSpeed
  (params (Speed :type Float%20%28double-precision%29))
  (Variables|/Script/Engine.CharacterMovementComponent|SetMaxWalkSpeed (Variables|Character|GetCharacterMovement) Speed))

(event Custom|RaggedyAnne
  (params (Origin :type Vector))
  (bind _mesh (Variables|Character|GetMesh))
  (Physics|SetSimulatePhysics _mesh true)
  (Physics|AddRadialImpulse _mesh (- Origin "0.000000,0.000000,-100.000000") 3e+02 7.5e+04 "RIF_Constant" false)
  (Pawn|Components|CharacterMovement|DisableMovement (Variables|Character|GetCharacterMovement)))

(event EventBeginPlay
  ;[0.15 0.15 0.15 0.5] Set body material as a variable
  (Variables|Default|SetOriginalMat (Rendering|Material|GetMaterial (Variables|Character|GetMesh) 0)))

(event Game|Damage|EventPointDamage
  (params (Damage :type Float%20%28single-precision%29) (DamageType :type Damage%20Type%20Object%20Reference) (HitLocation :type Vector :default "0, 0, 0") (HitNormal :type Vector :default "0, 0, 0") (HitComponent :type Primitive%20Component%20Object%20Reference) (BoneName :type Name :default "None") (ShotFromDirection :type Vector :default "0, 0, 0") (InstigatedBy :type Controller%20Object%20Reference) (DamageCauser :type Actor%20Object%20Reference) (HitInfo :type Hit%20Result%20Structure%20%28by%20ref%29))
  (Development|PrintText (Utilities|Text|FormatText "Instigator {INST} hit me for {DAM} damage" InstigatedBy Damage))
  (bind _output_get (Variables|Default|SetHealth (- (Variables|Default|GetHealth) Damage)))
  (if (<= _output_get 0.0)
    (Development|PrintString "Dead As Hell" true true "(R=1.000000,G=0.000000,B=0.164689,A=1.000000)")
    (CallFunction|RaggedyAnne ShotFromDirection)))

(fn ConstructionScript)

(fn GetPatrolPointLocation
  (bind _patrolroute (Variables|Default|GetPatrolRoute))
  (bind _spline (Variables|/Game/AI_Blueprints/BP_PatrolRoute.BP_PatrolRoute_C|GetSpline _patrolroute))
  (bind _output_get (Variables|Default|SetPatrolIndex (+ (Variables|Default|GetPatrolIndex) (Variables|Default|GetDirection))))
  (if (or (>= _output_get (- (Spline|GetNumberOfSplinePoints _spline) 1)) (<= (Variables|Default|GetPatrolIndex) 0))
    (Variables|Default|SetDirection (* (Variables|Default|GetDirection) -1)))
  (return (Spline|GetLocationatSplinePoint _spline (Variables|Default|GetPatrolIndex) "World")))

(fn GetIdealRange
  (return (Variables|Default|GetAttack%20Range) (Variables|Default|GetStrafe%20Range)))