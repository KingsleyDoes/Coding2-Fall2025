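; BP_PatrolRoute is a patrol route actor that supplies successive world-space waypoints from a spline, presumably for AI patrols.
; Each GetPatrolPointLocation call advances PatrolIndex by Direction and returns the location of that spline point.
; Direction flips once the index reaches zero or the point count, producing a back-and-forth route rather than a loop.
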(event EventBeginPlay)

(fn ConstructionScript)

(fn GetPatrolPointLocation
  (bind _output_get (Variables|Default|SetPatrolIndex (+ (Variables|Default|GetPatrolIndex) (Variables|Default|GetDirection))))
  (if (or (>= _output_get (Spline|GetNumberOfSplinePoints (Variables|Default|GetSpline))) (<= (Variables|Default|GetPatrolIndex) 0))
    (Variables|Default|SetDirection (* (Variables|Default|GetDirection) -1)))
  (return (Spline|GetLocationatSplinePoint (Variables|Default|GetSpline) (Variables|Default|GetPatrolIndex) "World")))